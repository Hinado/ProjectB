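; Blueprint from a tile-based game holding the win check that ends the game when only one faction remains.
; It gathers the unique factions of all Units not pending death.
; If exactly one is left, it shows the game-over HUD on the faction turn widget and sets GameOver on TB_GameMode.
; The winner text names the game mode's CurrentPawn faction rather than reading the surviving entry.
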(fn EndGameifOnlyOneFactionRemains
  (Utilities|Array|Clear (LocalVariables|GetRemaining%20Factions))
  (bind _outactors (Actor|GetAllActorsOfClass 0 "/Game/TileBased/Blueprints/Pawns/Unit.Unit_C"))
  (for _array_element _outactors
    (if (not (Variables|/Game/TileBased/Blueprints/Pawns/Unit.Unit_C|GetPending%20Death _array_element))
      (Utilities|Array|AddUnique (LocalVariables|GetRemaining%20Factions) (Variables|/Game/TileBased/Blueprints/Pawns/Unit.Unit_C|GetFaction _array_element))))
  (if (== (Utilities|Array|Length (LocalVariables|GetRemaining%20Factions)) 1)
    (bind _foundwidgets (Widget|GetAllWidgetsOfClass 0 "/Game/TileBased/Blueprints/Gameplay/Widgets/Widget_Faction_Turn.Widget_Faction_Turn_C"))
    (Rendering|Components|TextRender|SetText (Variables|/Game/TileBased/Blueprints/Gameplay/Widgets/Widget_Faction_Turn.Widget_Faction_Turn_C|Gettext_game_over (Utilities|Array|Get(acopy) _foundwidgets)) (Utilities|Text|ToText(String) (Utilities|String|Append (Class|KismetStringLibrary|ToUpper (Utilities|String|EnumtoString (Variables|/Game/TileBased/Blueprints/Pawns/Unit.Unit_C|GetFaction (Variables|/Game/TileBased/Blueprints/Gameplay/TB_GameMode.TB_GameMode_C|GetCurrentPawn (.AsTB%20Game%20Mode (Utilities|Casting|CastToTB_GameMode (Game|GetGameMode))))))) " FACTION WINS!")))
    (Default|GameOverHUD (Utilities|Array|Get(acopy) _foundwidgets))
    (Variables|/Game/TileBased/Blueprints/Gameplay/TB_GameMode.TB_GameMode_C|SetGame%20Over (.AsTB%20Game%20Mode (Utilities|Casting|CastToTB_GameMode (Game|GetGameMode))) true)
    (return)
    (else
      (return))))