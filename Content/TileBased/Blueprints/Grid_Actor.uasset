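; Base actor for objects on the tile grid, which works out its grid index and can snap to a custom grid at construction.
; The construction script finds the Grid_Manager and derives a 2D or 3D index from the actor's location, depending on the heightmap setting.
; With snapping on, it moves only the mesh anchor to the vector-field cell, unless a one-shot toggle also moves the actor there.
; Its interface functions return only default values.
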(fn ConstructionScript
  (bind _outactors (Actor|GetAllActorsOfClass "/Game/TileBased/Blueprints/Gameplay/Grid_Manager.Grid_Manager_C")) ; Get a referance to the Grid Manager
  (bind _output_get (Variables|Default|SetGridManagerRef (Utilities|Array|Get(acopy) _outactors)))
  (bind (_index _z) (Default|VectortoIndex3DNaive _output_get (Transformation|GetActorLocation)))
  (if (Utilities|Enum|Equal(Enum) (Variables|/Game/TileBased/Blueprints/Gameplay/Grid_Manager.Grid_Manager_C|GetHeightmap _output_get) "NewEnumerator3")
    (Variables|Default|SetIndex _index)
    (else
      (Variables|Default|SetIndex (Default|VectortoIndex2D _output_get (Transformation|GetActorLocation)))))
  (if (Variables|/Game/TileBased/Blueprints/Gameplay/Grid_Manager.Grid_Manager_C|GetSnapToCustomGrid (Variables|Default|GetGridManagerRef)) ; Is the Grid Manager set to snap to custom grid?
    (if (not (Variables|Default|GetIgnoreSnapToCustomGrid)) ; Should this specific actor ignore this?
      (Transformation|SetWorldLocation (Variables|Default|GetCustomGridAnchor) (Math|Vector|MakeVector (.x (+ (Utilities|Array|Get(acopy) (Variables|/Game/TileBased/Blueprints/Gameplay/Grid_Manager.Grid_Manager_C|GetVectorFieldArray (Variables|Default|GetGridManagerRef)) (Default|VectortoIndex2D _output_get (Transformation|GetActorLocation))) (Transformation|GetActorLocation (Variables|Default|GetGridManagerRef)))) (.y (+ (Utilities|Array|Get(acopy) (Variables|/Game/TileBased/Blueprints/Gameplay/Grid_Manager.Grid_Manager_C|GetVectorFieldArray (Variables|Default|GetGridManagerRef)) (Default|VectortoIndex2D _output_get (Transformation|GetActorLocation))) (Transformation|GetActorLocation (Variables|Default|GetGridManagerRef)))) _z) false false :!label _label) ; Set the location of the anchor which the mesh is tied to. Even though the actor is at the same position, the mesh will snap to the grid.
      (if (Variables|Default|GetPlace%20Actor%20at%20Anchor)
        (Transformation|SetActorLocation (Transformation|GetWorldLocation (Variables|Default|GetCustomGridAnchor)) false false) ; Places the actor at the same location as its anchor, which prevents it snapping back to its old position once grid snapping is turned off
        (Variables|Default|SetPlace%20Actor%20at%20Anchor false)
        (goto _label)))))

(fn GetVectorArrayInterface
  (params (Index :type Integer))
  (return "0, 0, 0"))

(fn MeshtoInstance
  (params (Actor :type Actor%20Object%20Reference))
  (return 0))

(fn VectortoIndexInterface
  (params (Vector :type Vector :default "0, 0, 0"))
  (return 0))